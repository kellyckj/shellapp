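; BP_Spectator is a spectator pawn that replicates its transform across the network.
; Each tick, a non-standalone, non-server instance sends its actor transform to the server through an RPC.
; The server stores it in PawnTransform, whose OnRep function sets the actor's transform without sweep or teleport.
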(event Custom|RPC%20Server%20Pawn%20Transform%20Replicate
  (params (transform :type Transform))
  ;[1 0.2685 0.3296] Server-side RPC Handling
  (Variables|Default|SetpawnTransform transform))

(event EventBeginPlay
  (Class|DDBlueprintLibrary|LogDebug "Spectator Pawn Begin Play"))

(event Collision|EventActorBeginOverlap
  (params (OtherActor :type Actor%20Object%20Reference)))

(event EventTick
  (params (DeltaSeconds :type Float%20%28single-precision%29))
  (Utilities|FlowControl|Sequence
    (:then_0
      ;[1 0.9635 0.1915] Replicate Pawn Transform by Calling RPC
      (if (and (not (Class|KismetSystemLibrary|IsStandalone)) (not (Networking|IsServer)))
        (CallFunction|RPCServerPawnTransformReplicate (Transformation|GetActorTransform))))))

(fn ConstructionScript)

(fn OnRepPawnTransform
  (Transformation|SetActorTransform (Variables|Default|GetpawnTransform)))